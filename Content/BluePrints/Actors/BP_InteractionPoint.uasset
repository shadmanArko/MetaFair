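; BP_InteractionPoint is an interaction point actor that shows a menu button prompt and can open a help desk UI.
; Its BoxCollider overlaps add a lazily created, reused UMG_MenuButton widget for BP_ThirdPersonCharacter and remove it on exit.
; Input is enabled at BeginPlay, so pressing Q creates a new UMG_HelpDesk and shows the mouse cursor, without any overlap check.
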(event OnComponentEndOverlap(BoxCollider)
  (params (OverlappedComponent :type Primitive%20Component%20Object%20Reference) (OtherActor :type Actor%20Object%20Reference) (OtherComp :type Primitive%20Component%20Object%20Reference) (OtherBodyIndex :type Integer))
  (Utilities|Casting|CastToBP_ThirdPersonCharacter OtherActor)
  (Development|PrintString "Exit")
  (Widget|RemovefromParent (Variables|Default|GetMenu%20Button%20Reference)))

(event OnComponentBeginOverlap(BoxCollider)
  (params (OverlappedComponent :type Primitive%20Component%20Object%20Reference) (OtherActor :type Actor%20Object%20Reference) (OtherComp :type Primitive%20Component%20Object%20Reference) (OtherBodyIndex :type Integer) (bFromSweep :type Boolean) (SweepResult :type Hit%20Result%20Structure%20%28by%20ref%29))
  (Utilities|Casting|CastToBP_ThirdPersonCharacter OtherActor)
  (Development|PrintString "enter")
  (Utilities|IsValid (Variables|Default|GetMenu%20Button%20Reference)
    (:Is%20Valid
      _)
    (:Is%20Not%20Valid
      (bind _returnvalue (UserInterface|CreateWidget "/Game/UMG/UMG_MenuButton.UMG_MenuButton_C"))
      (Variables|Default|SetMenu%20Button%20Reference _returnvalue)))
  (UserInterface|Viewport|AddtoViewport (Variables|Default|GetMenu%20Button%20Reference) 0))

(event EventBeginPlay
  (Input|EnableInput (Game|GetPlayerController 0)))

(event Collision|EventActorBeginOverlap
  (params (OtherActor :type Actor%20Object%20Reference)))

(event EventTick
  (params (DeltaSeconds :type Float%20%28single-precision%29)))

(event Input|KeyboardEvents|Q
  (params (Key :type Key%20Structure :default "None"))
  (:Pressed
    (bind _returnvalue (UserInterface|CreateWidget "/Game/UMG/UMG_HelpDesk.UMG_HelpDesk_C"))
    (UserInterface|Viewport|AddtoViewport _returnvalue 0)
    (Variables|/Script/Engine.PlayerController|SetbShowMouseCursor (Game|GetPlayerController 0) true)))

(fn ConstructionScript)